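; Leap Motion desktop-mode actor that drives left and right skeletal hand meshes from tracking data.
; On BeginPlay it sets desktop tracking, scales its origin by world-to-meters so hands keep a constant size, and assigns each mesh's anim class.
; Each tracking frame routes hand data by type into the matching low-poly stretch Anim Blueprint.
; The visibility-change events are empty, with their hide logic left disconnected.
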(event `self.ReceiveBeginPlay`
  (`LeapBlueprintFunctionLibrary.SetLeapMode` "LEAP_MODE_DESKTOP" "LEAP_SMOOTH")
  (`SceneComponent.SetRelativeScale3D` (`self.Origin`) (`KismetMathLibrary.Conv_DoubleToVector` (/ (`HeadMountedDisplayFunctionLibrary.GetWorldToMetersScale`) 100.0))) ; Hands are always same size
  (`SkeletalMeshComponent.SetAnimInstanceClass` (`SkeletalMeshActor.SkeletalMeshComponent` (`self.LeftHandSkeletalMesh`)) (`SkeletalMeshComponent.AnimClass` (`self.Left`)))
  (`SkeletalMeshComponent.SetAnimInstanceClass` (`SkeletalMeshActor.SkeletalMeshComponent` (`self.RightHandSkeletalMesh`)) (`SkeletalMeshComponent.AnimClass` (`self.Right`))))

(event `self.ReceiveEndPlay`
  (params (EndPlayReason :type "EEndPlayReason Enum" :default "Destroyed"))
  (`LeapBlueprintFunctionLibrary.SetLeapMode` "LEAP_MODE_DESKTOP" "LEAP_SMOOTH"))

(event `self.Leap.OnLeapTrackingData`
  (params (Frame :type "LeapFrameData Structure (by ref)"))
  (for _array_element (`.Hands` (break `LeapFrameData` Frame))
    ;[1 1 1] Set Animation Data for each hand
    (switch `EHandType` (`.HandType` (break `LeapHandData` _array_element))
      (:`LEAP_HAND_LEFT`
        (`self.SetLeftAnim` _array_element))
      (:`LEAP_HAND_RIGHT`
        (`self.SetRightAnim` _array_element)))))

(event `self.Leap.OnLeftHandVisibilityChanged`
  (params (bIsVisible :type Boolean))
  ;[1 1 1] Sync mesh visibility with tracking visibility updates
)

(event `self.Leap.OnRightHandVisibilityChanged`
  (params (bIsVisible :type Boolean))
  ;[1 1 1] Sync mesh visibility with tracking visibility updates
)

(fn `SetLeftAnim`
  (params (HandData :type "LeapHandData Structure"))
  (bind _asleap_low_poly_left_stretch_anim_bp (cast `/LeapMotion/DirectRigging/LowPoly/LeapLowPolyLeftStretchAnimBP` (`SkeletalMeshComponent.GetAnimInstance` (`SkeletalMeshActor.SkeletalMeshComponent` (`self.LeftHandSkeletalMesh`)))))
  (`/LeapMotion/DirectRigging/LowPoly/LeapLowPolyLeftStretchAnimBP.SetAnimData` _asleap_low_poly_left_stretch_anim_bp HandData))

(fn `SetRightAnim`
  (params (HandData :type "LeapHandData Structure"))
  (bind _asleap_low_poly_right_stretch_anim_bp (cast `/LeapMotion/DirectRigging/LowPoly/LeapLowPolyRightStretchAnimBP` (`SkeletalMeshComponent.GetAnimInstance` (`SkeletalMeshActor.SkeletalMeshComponent` (`self.RightHandSkeletalMesh`)))))
  (`/LeapMotion/DirectRigging/LowPoly/LeapLowPolyRightStretchAnimBP.SetAnimData` _asleap_low_poly_right_stretch_anim_bp HandData))

(fn `UserConstructionScript`)